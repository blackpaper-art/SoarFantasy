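; BP_DeathGround is a ground hazard that toggles the player's stuck state through two overlap zones.
; On BeginPlay it caches the player pawn as CharactersKix and binds overlap events on GroundDeadZone and GroundRepair.
; When the player enters GroundDeadZone, it zeroes the movement plane constraint normal and calls MakeStuck(true).
; Entering GroundRepair sets the normal back to the X axis and clears the stuck state.
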(event `self.ReceiveBeginPlay`
  (`|ExecutionSequence`
    (:`then_0`
      (bind _ascharacters_kix (cast `CharactersKix` (`GameplayStatics.GetPlayerPawn` 0)))
      (set `self.As Characters Kix` _ascharacters_kix))
    (:`then_1`
      (add `PrimitiveComponent.OnComponentBeginOverlap` (`self.GroundDeadZone`) (delegate `OnComponentBeginOverlap_Event`)))
    (:`then_2`
      (add `PrimitiveComponent.OnComponentBeginOverlap` (`self.GroundRepair`) (delegate `OnComponentBeginOverlap_Event_0`)))))

(event `OnComponentBeginOverlap_Event`
  (params (OverlappedComponent :type "PrimitiveComponent Object Reference") (OtherActor :type "Actor Object Reference") (OtherComp :type "PrimitiveComponent Object Reference") (OtherBodyIndex :type Integer) (bFromSweep :type Boolean) (SweepResult :type "HitResult Structure (by ref)"))
  (bind _as_characters_kix (`self.As Characters Kix`))
  (if (== _as_characters_kix OtherActor)
    (`MovementComponent.SetPlaneConstraintNormal` (`Character.CharacterMovement` _as_characters_kix) (0.0 0.0 0.0))
    (`CharactersKix.MakeStuck` _as_characters_kix true)))

(event `OnComponentBeginOverlap_Event_0`
  (params (OverlappedComponent :type "PrimitiveComponent Object Reference") (OtherActor :type "Actor Object Reference") (OtherComp :type "PrimitiveComponent Object Reference") (OtherBodyIndex :type Integer) (bFromSweep :type Boolean) (SweepResult :type "HitResult Structure (by ref)"))
  (bind _as_characters_kix (`self.As Characters Kix`))
  (if (== _as_characters_kix OtherActor)
    (`MovementComponent.SetPlaneConstraintNormal` (`Character.CharacterMovement` _as_characters_kix) (1.0 0.0 0.0))
    (`CharactersKix.MakeStuck` _as_characters_kix false)))

(fn `UserConstructionScript`)