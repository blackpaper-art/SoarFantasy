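; BP_ConeEnemy is a cone enemy hazard that kills the player's Kix character on contact.
; On BeginPlay it caches the player pawn as CharactersKix and binds an overlap event to its BoxSphereDeadZone component.
; When that same character enters the zone, it calls KixDead on it; other actors are ignored.
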(event `self.ReceiveBeginPlay`
  (`|ExecutionSequence`
    (:`then_0`
      (bind _ascharacters_kix (cast `CharactersKix` (`GameplayStatics.GetPlayerPawn` 0)))
      (set `self.As Characters Kix` _ascharacters_kix))
    (:`then_1`
      (add `PrimitiveComponent.OnComponentBeginOverlap` (`self.BoxSphereDeadZone`) (delegate `OnBoxDeadZoneBeginOverlap_Event`)))))

(event `OnBoxDeadZoneBeginOverlap_Event`
  (params (OverlappedComponent :type "PrimitiveComponent Object Reference") (OtherActor :type "Actor Object Reference") (OtherComp :type "PrimitiveComponent Object Reference") (OtherBodyIndex :type Integer) (bFromSweep :type Boolean) (SweepResult :type "HitResult Structure (by ref)"))
  (bind _as_characters_kix (`self.As Characters Kix`))
  (if (== OtherActor _as_characters_kix)
    (`CharactersKix.KixDead` _as_characters_kix)))

(fn `UserConstructionScript`)