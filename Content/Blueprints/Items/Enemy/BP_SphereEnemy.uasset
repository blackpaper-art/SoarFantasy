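; BP_SphereEnemy is a stompable enemy that kills the player on contact or dies when jumped on.
; On BeginPlay it caches the player pawn as CharactersKix and binds overlap events to two zones.
; Overlapping the box dead zone calls KixDead on the player.
; Overlapping the sphere jump zone launches the player upward, destroys the enemy and plays a sound.
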(event `self.ReceiveBeginPlay`
  (`|ExecutionSequence`
    (:`then_0`
      (bind _ascharacters_kix (cast `CharactersKix` (`GameplayStatics.GetPlayerPawn` 0)))
      (set `self.As Characters Kix` _ascharacters_kix))
    (:`then_1`
      (add `PrimitiveComponent.OnComponentBeginOverlap` (`self.BoxSphereDeadZone`) (delegate `OnBoxDeadZoneBeginOverlap_Event`)))
    (:`then_2`
      (add `PrimitiveComponent.OnComponentBeginOverlap` (`self.SphereJumpZone`) (delegate `OnJumpZoneBeginOverlap_Event`)))))

(event `OnBoxDeadZoneBeginOverlap_Event`
  (params (OverlappedComponent :type "PrimitiveComponent Object Reference") (OtherActor :type "Actor Object Reference") (OtherComp :type "PrimitiveComponent Object Reference") (OtherBodyIndex :type Integer) (bFromSweep :type Boolean) (SweepResult :type "HitResult Structure (by ref)"))
  (bind _as_characters_kix (`self.As Characters Kix`))
  (if (== OtherActor _as_characters_kix)
    (`CharactersKix.KixDead` _as_characters_kix)))

(event `OnJumpZoneBeginOverlap_Event`
  (params (OverlappedComponent :type "PrimitiveComponent Object Reference") (OtherActor :type "Actor Object Reference") (OtherComp :type "PrimitiveComponent Object Reference") (OtherBodyIndex :type Integer) (bFromSweep :type Boolean) (SweepResult :type "HitResult Structure (by ref)"))
  (bind _as_characters_kix (`self.As Characters Kix`))
  (if (== OtherActor _as_characters_kix)
    (`Character.LaunchCharacter` _as_characters_kix (0.0 0.0 600.0) true true)
    (`self.K2_DestroyActor`)
    (`GameplayStatics.PlaySound2D` "/Game/Assets/Sounds/Enemy/JumpForEnemy.JumpForEnemy" 1.0 1.0 0.0 null null)))

(fn `UserConstructionScript`)