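; BP_MapSpawner builds the level from the DT_Map data table on BeginPlay.
; Each row becomes a column along X, with its platform, air and coin layers stacked along Z using the spacing variables.
; Each layer value is looked up in ActorMap for the class to spawn, and every spawn receives a CoinCount converted from the coin layer.
; GenerateCoins is an unfinished stub.
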(event `self.ReceiveBeginPlay`
  (`self.GenerateMaps`))

(fn `GenerateCoins`
  (`DataTableFunctionLibrary.GetDataTableRowNames` "/Game/Blueprints/Generaters/MapData/DT_Map.DT_Map"))

(fn `GenerateMaps`
  (bind _outrownames (`DataTableFunctionLibrary.GetDataTableRowNames` "/Game/Blueprints/Generaters/MapData/DT_Map.DT_Map"))
  (for (_array_element _array_index) _outrownames
    (bind _returnvalue (`|GetDataTableRow` "/Game/Blueprints/Generaters/MapData/DT_Map.DT_Map" _array_element)
      (:`then`
        (bind (_platform_layer _air_layer _coin_layer) (break `/Game/Blueprints/Generaters/MapData/S_MapContext` _returnvalue))
        (for (_array_element_2 _array_index_2) (`|MakeArray` _platform_layer _air_layer _coin_layer)
          (bind _output_get (set `self.GeneratLoc` (`KismetMathLibrary.MakeVector` (* _array_index (`self.YSpace`)) 0.0 (* _array_index_2 (`self.XSpace`)))))
          (`|SpawnActorFromClass` (`|ConvertAsset` (`BlueprintMapLibrary.Map_Find` (`self.ActorMap`) _array_element_2)) (`KismetMathLibrary.MakeTransform` _output_get) "Undefined" "MultiplyWithRoot" null 0.0 (`KismetStringLibrary.Conv_StringToInt` _coin_layer) null))))))

(fn `UserConstructionScript`)